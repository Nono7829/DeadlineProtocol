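; Test enemy character that roams the navmesh, chases the player and plays a melee attack montage on reaching them.
; PawnSensing sightings start an AI MoveTo chase, with a CanAttack flag gating the montage.
; After the montage's duration it clears IsSeeingPlayer and resumes chained random moves around itself until the next sighting.
; AnyDamage subtracts from Health while positive, with no death handling.
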(event `self.ReceiveAnyDamage`
  (params (Damage :type "Float (single-precision)") (DamageType :type "DamageType Object Reference") (InstigatedBy :type "Controller Object Reference") (DamageCauser :type "Actor Object Reference"))
  (if (> (`self.Health`) 0.0)
    (set `self.Health` (- (`self.Health`) Damage))))

(event `FollowPlayer`
  (set `self.CanAttack?` true :!label _label)
  (if (`self.IsSeeingPlayer?`)
    (`|AIMoveTo` self (0.0 0.0 0.0) (`GameplayStatics.GetPlayerCharacter` 0) 70.0
      (:`OnSuccess`
        (if (`self.CanAttack?`)
          (set `self.CanAttack?` false)
          (bind _returnvalue (`self.PlayAnimMontage` "/Game/Characters/Mannequins/Anims/AM_Paired_CounterPunch_PalmStrike_Att_Montage.AM_Paired_CounterPunch_PalmStrike_Att_Montage"))
          (`KismetSystemLibrary.Delay` _returnvalue)
          (set `self.IsSeeingPlayer?` false)
          (if (`self.IsSeeingPlayer?`) :!label _label_2
            (set `self.IsSeeingPlayer?` true :!label _label_3)
            (goto _label)
            (else
              (set `self.IsSeeingPlayer?` false :!label _label_4)
              (bind _randomlocation (`NavigationSystemV1.K2_GetRandomLocationInNavigableRadius` (`self.K2_GetActorLocation`) 500.0 null null :!label _label_5))
              (`|AIMoveTo` self _randomlocation null
                (:`OnSuccess`
                  (goto _label_5))))))))
    (else
      (goto _label_4))))

(event `self.PawnSensing.OnSeePawn`
  (params (Pawn :type "Pawn Object Reference"))
  (goto _label_3))

(event `self.ReceiveBeginPlay`
  (goto _label_2))

(fn `UserConstructionScript`)