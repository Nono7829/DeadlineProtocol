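; Pistol bullet projectile that sticks into static surfaces and drops off anything else as a physics object.
; On hit it disables collision; against static geometry it snaps to face into the surface, wiggles the Sphere via a timeline, then falls after a short delay.
; Stationary or movable hits zero velocity and enable physics immediately.
; The parent Hit logic always follows, and projectile bounces only print a debug string.
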(event `self.ReceiveHit`
  (params (MyComp :type "PrimitiveComponent Object Reference") (Other :type "Actor Object Reference") (OtherComp :type "PrimitiveComponent Object Reference") (bSelfMoved :type Boolean) (HitLocation :type "Vector Structure") (HitNormal :type "Vector Structure") (NormalImpulse :type "Vector Structure") (Hit :type "HitResult Structure (by ref)"))
  (`|ExecutionSequence`
    (:`then_0`
      (`PrimitiveComponent.SetCollisionEnabled` (`self.CollisionComponent`) "NoCollision")
      (switch `EComponentMobility` (`SceneComponent.Mobility` OtherComp)
        (:`Static`
          (`self.K2_SetActorLocationAndRotation` HitLocation (`KismetMathLibrary.MakeRotFromX` (* HitNormal -1.0)))
          (bind (_direction _newtrack_0) (`Timeline|Wiggle`)
            (:`Update`
              (`SceneComponent.K2_AddRelativeRotation` (`self.Sphere`) (`KismetMathLibrary.MakeRotator` (* _newtrack_0 3.0)) false false))
            (:`Finished`
              (`KismetSystemLibrary.Delay` 3.0)
              (`PrimitiveComponent.SetPhysicsLinearVelocity` (`self.Sphere`) (0.0 0.0 0.0) false "None" :!label _label)
              (`PrimitiveComponent.SetSimulatePhysics` (`self.Sphere`) true))))
        (:`Stationary`
          (goto _label))
        (:`Movable`
          (goto _label))))
    (:`then_1`
      (`parent.ReceiveHit` MyComp Other OtherComp bSelfMoved HitLocation HitNormal NormalImpulse Hit))))

(event `self.ProjectileMovement.OnProjectileBounce`
  (params (ImpactResult :type "HitResult Structure (by ref)") (ImpactVelocity :type "Vector Structure (by ref)"))
  (`KismetSystemLibrary.PrintString` "Hello"))

(fn `UserConstructionScript`
  (`parent.UserConstructionScript`))