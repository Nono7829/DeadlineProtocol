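; BP_Medkit is a health pickup that restores an overlapping BP_FirstPersonCharacter to full health and then destroys itself.
; BoxCollider overlap shows the Widget for any actor, then casts to the character, writes the missing health to its AmountHeatlh variable and adds that to Health.
; The new Health value is printed as debug output, and ending the overlap hides the Widget.
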(event `self.Box Collider.OnComponentBeginOverlap`
  (params (OverlappedComponent :type "PrimitiveComponent Object Reference") (OtherActor :type "Actor Object Reference") (OtherComp :type "PrimitiveComponent Object Reference") (OtherBodyIndex :type Integer) (bFromSweep :type Boolean) (SweepResult :type "HitResult Structure (by ref)"))
  (`SceneComponent.SetVisibility` (`self.Widget`) true false)
  (bind _asbp_first_person_character (cast `/Game/FirstPerson/Blueprints/BP_FirstPersonCharacter` OtherActor))
  (bind _output_get (set `/Game/FirstPerson/Blueprints/BP_FirstPersonCharacter.AmountHeatlh` (- (`/Game/FirstPerson/Blueprints/BP_FirstPersonCharacter.MaxHealth` _asbp_first_person_character) (`/Game/FirstPerson/Blueprints/BP_FirstPersonCharacter.Health` _asbp_first_person_character)) _asbp_first_person_character))
  (bind _output_get_2 (set `/Game/FirstPerson/Blueprints/BP_FirstPersonCharacter.Health` (+ (`/Game/FirstPerson/Blueprints/BP_FirstPersonCharacter.Health` _asbp_first_person_character) _output_get) _asbp_first_person_character))
  (`self.K2_DestroyActor`)
  (`KismetSystemLibrary.PrintString` (`KismetStringLibrary.Conv_DoubleToString` _output_get_2)))

(event `self.Box Collider.OnComponentEndOverlap`
  (params (OverlappedComponent :type "PrimitiveComponent Object Reference") (OtherActor :type "Actor Object Reference") (OtherComp :type "PrimitiveComponent Object Reference") (OtherBodyIndex :type Integer))
  (`SceneComponent.SetVisibility` (`self.Widget`) false false))

(fn `UserConstructionScript`)